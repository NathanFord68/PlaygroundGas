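; GA_HurtTarget is a Gameplay Ability that damages a pawn just in front of the avatar.
; On activation it commits the ability, cancelling if that fails.
; It then runs a short forward sphere trace for pawns, ignoring the avatar and drawing debug.
; The hit actor becomes target data for GE_Damage, applied without checking the hit, and the ability ends.
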(event Ability|EventActivateAbility
  (bind _returnvalue (Ability|GetAvatarActorfromActorInfo))
  (bind _returnvalue_2 (Transformation|GetActorLocation _returnvalue))
  ;[0.15 0.15 0.15 0.5] Starts the ability, CommitAbility can return false if we cannot commit. If this is the case we must cancel the ability system so GAS knows we're not doing it anymore
  (bind _returnvalue_3 (Ability|CommitAbility))
  (if _returnvalue_3
    ;[0.15 0.15 0.15 0.5] Standard Ray trace to get the actor that we're looking at. Not a GAS thing but we do need it so we know who we're trying to apply the effect to
    (bind _outhit (Collision|SphereTraceForObjects _returnvalue_2 (+ _returnvalue_2 (* (Transformation|GetActorForwardVector _returnvalue) 1e+02)) 0.0 (Utilities|Array|MakeArray "ObjectTypeQuery3") false (Utilities|Array|MakeArray _returnvalue) "ForDuration"))
    ;[0.15 0.15 0.15 0.5] Applies the effect we just created to the target we hit
    (GameplayEffects|ApplyGameplayEffectToTarget (Ability|TargetData|AbilityTargetDatafromActor (.HitActor (Collision|BreakHitResult _outhit))) "/Game/Effects/GE_Damage.GE_Damage_C" 1 1)
    (Ability|EndAbility) ; Let's the system know we're done
    (else
      (Ability|CancelAbility))))