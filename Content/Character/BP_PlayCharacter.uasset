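; BP_PlayCharacter is a player character that moves, aims and triggers a hurt-target ability.
; On BeginPlay it caches its PlayerController, adds the default Enhanced Input mapping context and grants GA_HurtTarget through its AbilitySystemComponent.
; The hurt-target input activates the granted ability by its stored handle.
; Move input follows the controller's forward and right vectors, while aim input drives controller yaw and pitch.
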(event Input|EnhancedActionEvents|EnhancedInputActionIA_Move
  (params (ActionValue :type Vector%202D%20Structure) (ElapsedSeconds :type Float%20%28double-precision%29) (TriggeredSeconds :type Float%20%28double-precision%29) (InputAction :type Input%20Action%20Object%20Reference :default "/Game/Input/Actions/IA_Move.IA_Move"))
  (bind _as_player_controller (Variables|Default|GetAs%20Player%20Controller))
  (Pawn|Input|AddMovementInput (+ (* (Transformation|GetActorForwardVector _as_player_controller) (.x ActionValue)) (* (Transformation|GetActorRightVector _as_player_controller) (.y ActionValue))) 1.0 false))

(event Input|EnhancedActionEvents|EnhancedInputActionIA_Aim
  (params (ActionValue :type Vector%202D%20Structure) (ElapsedSeconds :type Float%20%28double-precision%29) (TriggeredSeconds :type Float%20%28double-precision%29) (InputAction :type Input%20Action%20Object%20Reference :default "/Game/Input/Actions/IA_Aim.IA_Aim"))
  (Pawn|Input|AddControllerYawInput (.x ActionValue))
  (bind _result (Math|Float|NegateFloat (.y ActionValue))
    (:%20%20
      (Pawn|Input|AddControllerPitchInput _result))))

(event Input|EnhancedActionEvents|EnhancedInputActionIA_HurtTarget
  (params (ActionValue :type Boolean) (ElapsedSeconds :type Float%20%28double-precision%29) (TriggeredSeconds :type Float%20%28double-precision%29) (InputAction :type Input%20Action%20Object%20Reference :default "/Game/Input/Actions/IA_HurtTarget.IA_HurtTarget"))
  (Class|AbilitySystemComponent|TryActivateAbility (Variables|Default|GetAbilitySystemComponent) (stale EventBeginPlay _returnvalue) true))

(event EventBeginPlay
  (bind _asplayer_controller (Utilities|Casting|CastToPlayerController (Pawn|GetController)))
  (bind _output_get (Variables|Default|SetAs%20Player%20Controller _asplayer_controller))
  (Input|AddMappingContext (PlayerController|LocalPlayerSubsystems|GetEnhancedInputLocalPlayerSubsystem _output_get) "/Game/Input/Mappings/IMC_Default.IMC_Default" 0 "(bIgnoreAllPressedKeysUntilRelease=True,bForceImmediately=False,bNotifyUserSettings=False)")
  (bind _returnvalue (GameplayAbilities|GiveAbility (Variables|Default|GetAbilitySystemComponent) "/Game/Abilities/GA_HurtTarget.GA_HurtTarget_C" 0 -1)))

(fn ConstructionScript)